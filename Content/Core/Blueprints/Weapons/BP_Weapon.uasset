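; Weapon Blueprint that fires BP_Projectile from the mesh's Muzzle socket, with the owning Character as instigator.
; For a locally controlled character, StartFire opens a Gate that loops shots every FireRate through a retriggerable delay and ContinueFire until StopFire closes it.
; Otherwise StartFire fires once.
; Each shot passes muzzle rotation to ReplicateFire, and SimulateFire spawns a projectile using a supplied rotation.
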(event EventStartFire
  (bind _mesh (Variables|Character|GetMesh))
  (bind _mesh_2 (Variables|Character|GetMesh))
  (bind _returnvalue (Transformation|GetSocketTransform _mesh_2 "Muzzle" "RTS_World"))
  (bind _returnvalue_2 (Transformation|GetSocketTransform _mesh "Muzzle" "RTS_World"))
  (if (Pawn|IsLocallyControlled (Variables|Default|GetCharacter))
    (Utilities|FlowControl|Sequence
      (:then_0
        (goto _label Open))
      (:then_1
        (Utilities|FlowControl|Gate true :!label _label
          (:Exit
            (Game|SpawnActorfromClass "/Game/Core/Blueprints/Projectile/BP_Projectile.BP_Projectile_C" (Math|Transform|MakeTransform (.location _returnvalue) (.rotation _returnvalue)) "Undefined" "MultiplyWithRoot" 0 (Variables|Default|GetCharacter))
            (Class|ZoneProjectWeapon|ReplicateFire (.rotation _returnvalue))
            (Utilities|FlowControl|RetriggerableDelay (Variables|Default|GetFireRate))
            (Class|ZoneProjectWeapon|ContinueFire)))))
    (else
      (Game|SpawnActorfromClass "/Game/Core/Blueprints/Projectile/BP_Projectile.BP_Projectile_C" (Math|Transform|MakeTransform (.location _returnvalue_2) (.rotation _returnvalue_2)) "Undefined" "MultiplyWithRoot" 0 (Variables|Default|GetCharacter))
      (Class|ZoneProjectWeapon|ReplicateFire (.rotation _returnvalue_2)))))

(event EventContinueFire
  (bind _mesh (Variables|Character|GetMesh))
  (bind _returnvalue (Transformation|GetSocketTransform _mesh "Muzzle" "RTS_World"))
  (Utilities|FlowControl|Gate true
    (:Exit
      (Game|SpawnActorfromClass "/Game/Core/Blueprints/Projectile/BP_Projectile.BP_Projectile_C" (Math|Transform|MakeTransform (.location _returnvalue) (.rotation _returnvalue)) "Undefined" "MultiplyWithRoot" 0 (Variables|Default|GetCharacter))
      (Class|ZoneProjectWeapon|ReplicateFire (.rotation _returnvalue))
      (Utilities|FlowControl|RetriggerableDelay (Variables|Default|GetFireRate))
      (Class|ZoneProjectWeapon|ContinueFire))))

(event EventStopFire
  (bind _mesh (Variables|Character|GetMesh))
  (bind _returnvalue (Transformation|GetSocketTransform _mesh "Muzzle" "RTS_World"))
  (Utilities|FlowControl|Gate true) ; enters at Close
)

(event EventSimulateFire
  (params (Rotation :type Rotator :default "0, 0, 0"))
  (Game|SpawnActorfromClass "/Game/Core/Blueprints/Projectile/BP_Projectile.BP_Projectile_C" (Math|Transform|MakeTransform (.location (Transformation|GetSocketTransform (Variables|Character|GetMesh) "Muzzle" "RTS_World")) Rotation) "Undefined" "MultiplyWithRoot" 0 (Variables|Default|GetCharacter)))

(fn ConstructionScript)