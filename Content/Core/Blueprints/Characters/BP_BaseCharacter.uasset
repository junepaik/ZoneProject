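; Base character Blueprint that drifts its camera ahead of the direction the character faces.
; Each Tick eases the CameraBoom's target offset toward a fixed-distance point along the actor's forward vector, plus a constant Y shift, using a slow VInterpTo.
; An unconnected node chain would scale that look-ahead by clamped forward speed; BeginPlay and the construction script are empty.
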(event EventBeginPlay)

(event EventTick
  (params (DeltaSeconds :type Float%20%28single-precision%29))
  (bind _cameraboom (Variables|Default|GetCameraBoom))
  (Variables|/Script/Engine.SpringArmComponent|SetTargetOffset _cameraboom (Math|Interpolation|VInterpTo (Variables|/Script/Engine.SpringArmComponent|GetTargetOffset _cameraboom) (+ (* (Math|Vector|GetForwardVector (Transformation|GetActorRotation)) 2e+02) "0.000000,100.000000,0.000000") (Utilities|Time|GetWorldDeltaSeconds) 0.5)))

(fn ConstructionScript)